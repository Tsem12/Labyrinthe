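; BP_WinGate is a gate in the labyrinth game that opens or closes according to an Active flag.
; On BeginPlay it caches the Cube's world transform as the closed state and derives the open state by raising it along Z.
; MoveGate teleports the Cube to either transform without animation and swaps its material between the enabled and disabled module looks.
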(event EventBeginPlay
  ;[1 1 1] Set closed transform
  (bind _output_get (Variables|Default|SetClosedTrasform (Transformation|GetWorldTransform (Variables|Default|GetCube))))
  ;[1 1 1] Set open Transform
  (Variables|Default|SetOpenTransform (Math|Transform|MakeTransform (+ (.location _output_get) "0.000000,0.000000,590.000000") (.rotation _output_get) (.scale _output_get))))

(fn ConstructionScript)

(fn MoveGate
  (params (Active :type Boolean))
  (bind _cube (Variables|Default|GetCube))
  ;[1 1 1] Comment
  (if Active
    (Transformation|SetWorldTransform _cube (Variables|Default|GetOpenTransform) false true)
    (Rendering|Material|SetMaterial _cube 0 "/Engine/EditorMaterials/Cascade/CASC_ModuleEnable_MAT.CASC_ModuleEnable_MAT")
    (else
      (Transformation|SetWorldTransform _cube (Variables|Default|GetClosedTrasform) false true)
      (Rendering|Material|SetMaterial _cube 0 "/Engine/EditorMaterials/Cascade/CASC_ModuleDisable_MAT.CASC_ModuleDisable_MAT"))))